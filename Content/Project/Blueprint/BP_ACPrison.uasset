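; BP_ACPrison is a prison actor that animates its swinging cell door, supplied by a BP_ACPrisonDoor child actor.
; On BeginPlay it caches the child's pivot and door components.
; OnDoorStateChanged plays or reverses a timeline that sets the pivot's relative yaw.
; Door collision is disabled when opening starts and restored when the timeline finishes.
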(event EventBeginPlay
  (bind _asbp_acprison_door (Utilities|Casting|CastToBP_ACPrisonDoor (Variables|/Script/Engine.ChildActorComponent|GetChildActor (Variables|Default|GetBP_ACPrisonDoor))))
  (Variables|Default|SetPivot%20Door%20Ref (Variables|/Game/Project/Blueprint/BP_ACPrisonDoor.BP_ACPrisonDoor_C|GetPivot_Door _asbp_acprison_door))
  (Variables|Default|SetPrison%20Door%20Ref (Variables|/Game/Project/Blueprint/BP_ACPrisonDoor.BP_ACPrisonDoor_C|GetPrison_Door _asbp_acprison_door)))

(event EventOnDoorStateChanged
  (params (bOpen :type Boolean))
  (if bOpen
    (Collision|SetCollisionEnabled (Variables|Default|GetPrison%20Door%20Ref) "NoCollision")
    (bind _doorangle (Timeline|TL_DoorRotation PlayFromStart)
      (:Update
        (Transformation|SetRelativeRotation (Variables|Default|GetPivot%20Door%20Ref) (Math|Rotator|MakeRotator 0.0 0.0 _doorangle) false false))
      (:Finished
        (Collision|SetCollisionEnabled (Variables|Default|GetPrison%20Door%20Ref) "QueryAndPhysics")))
    (else
      (Timeline|TL_DoorRotation ReverseFromEnd))))

(fn ConstructionScript)