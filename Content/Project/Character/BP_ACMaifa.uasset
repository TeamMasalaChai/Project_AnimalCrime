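; BP_ACMaifa is a character Blueprint that handles camera modes, starting in third person.
; IA_CameraMode flip-flops between TPS and FPS child-actor cameras using blended view targets, hiding or showing face, head and body meshes after the blend delay.
; IA_Zoom, active only in TPS mode, blends to a zoom camera once per press through a DoOnce, then returns and resets on release or cancel.
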(event Input|EnhancedActionEvents|EnhancedInputActionIA_CameraMode
  (params (ActionValue :type Boolean) (ElapsedSeconds :type Float%20%28double-precision%29) (TriggeredSeconds :type Float%20%28double-precision%29) (InputAction :type Input%20Action%20Object%20Reference :default "/Game/Project/Input/Actions/IA_CameraMode.IA_CameraMode"))
  (:Started
    (Utilities|FlowControl|FlipFlop
      (:A
        (Variables|Default|SetIsTPSMode false)
        (Game|Player|SetViewTargetwithBlend (Game|GetPlayerController 0) (Variables|/Script/Engine.ChildActorComponent|GetChildActor (Variables|Default|GetFPSCamera)) (Variables|Default|GetCameraBlendTime) "VTBlend_Linear" 0.0 false)
        (Utilities|FlowControl|Delay (Variables|Default|GetCameraBlendTime))
        (Development|SetHiddeninGame (Variables|Default|GetFaceMesh) true true))
      (:B
        (Variables|Default|SetIsTPSMode true)
        (Game|Player|SetViewTargetwithBlend (Game|GetPlayerController 0) (Variables|/Script/Engine.ChildActorComponent|GetChildActor (Variables|Default|GetTPSCamera)) (Variables|Default|GetCameraBlendTime) "VTBlend_Linear" 0.0 false)
        (Utilities|FlowControl|Delay (Variables|Default|GetCameraBlendTime))
        (Development|SetHiddeninGame (Variables|Default|GetHeadMesh) false true)))))

(event Input|EnhancedActionEvents|EnhancedInputActionIA_Zoom
  (params (ActionValue :type Boolean) (ElapsedSeconds :type Float%20%28double-precision%29) (TriggeredSeconds :type Float%20%28double-precision%29) (InputAction :type Input%20Action%20Object%20Reference :default "/Game/Project/Input/Actions/IA_Zoom.IA_Zoom"))
  (:Triggered
    (if (Variables|Default|GetIsTPSMode)
      (Utilities|FlowControl|DoOnce false :!label _label
        (:Completed
          (Game|Player|SetViewTargetwithBlend (Game|GetPlayerController 0) (Variables|/Script/Engine.ChildActorComponent|GetChildActor (Variables|Default|GetTPSZoomCamera)) (Variables|Default|GetCameraBlendTime) "VTBlend_Linear" 0.0 false)
          (Variables|Default|SetIsZoomed true)))))
  (:Canceled
    (if (Variables|Default|GetIsTPSMode) :!label _label_2
      (Game|Player|SetViewTargetwithBlend (Game|GetPlayerController 0) (Variables|/Script/Engine.ChildActorComponent|GetChildActor (Variables|Default|GetTPSCamera)) (Variables|Default|GetCameraBlendTime) "VTBlend_Linear" 0.0 false)
      (Variables|Default|SetIsZoomed false)
      (goto _label Reset)))
  (:Completed
    (goto _label_2)))

(event EventBeginPlay
  ;[0.15 0.15 0.15 0.5] 기본 카메라 세팅
  (Game|Player|SetViewTargetwithBlend (Game|GetPlayerController 0) (Variables|/Script/Engine.ChildActorComponent|GetChildActor (Variables|Default|GetTPSCamera)) 0.0 "VTBlend_Linear" 0.0 false)
  (Variables|Default|SetIsTPSMode true))

(event Collision|EventActorBeginOverlap
  (params (OtherActor :type Actor%20Object%20Reference)))

(event EventTick
  (params (DeltaSeconds :type Float%20%28single-precision%29)))

(fn ConstructionScript)